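; Game mode for a Minesweeper game that sets up the camera, mouse input and HUD, and handles score updates and game over.
; On BeginPlay it views through the first BP_Grid, enables cursor with click and hover events, creates the GameUI widget and refreshes scores per grid.
; UpdateScores writes the grid's remaining bomb and tile counts to the widget.
; GameOver plays an explosion camera shake at the bomb tile's location.
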(event `self.ReceiveBeginPlay`
  (bind _returnvalue (`GameplayStatics.GetPlayerController` 0))
  ;[1 1 1] Set Up Camera
  (bind _outactors (`GameplayStatics.GetAllActorsOfClass` "/Game/BP_Grid.BP_Grid_C"))
  (`PlayerController.SetViewTargetWithBlend` _returnvalue (`|GetArrayItem` _outactors) 0.0 "VTBlend_Linear" 0.0 false)
  ;[1 1 1] Set Up Mouse Input
  (set `PlayerController.bEnableMouseOverEvents` true _returnvalue)
  (set `PlayerController.bEnableClickEvents` true _returnvalue)
  (set `PlayerController.bShowMouseCursor` true _returnvalue)
  ;[1 1 1] Set up Game UI
  (bind _returnvalue_2 (`|CreateWidget` "/Game/GameUI.GameUI_C"))
  (bind _output_get (set `self.GameUIWidget` _returnvalue_2))
  (`UserWidget.AddToViewport` _output_get 0)
  (bind _outactors_2 (`GameplayStatics.GetAllActorsOfClass` "/Game/BP_Grid.BP_Grid_C"))
  (for _array_element _outactors_2
    (`self.UpdateScores` _array_element)))

(event `UpdateScores`
  (params (GameGrid :type "/Game/BP_Grid Object Reference"))
  (bind _gameuiwidget (`self.GameUIWidget`))
  ;[1 1 1] Update Scores
  (bind (_bombsremaining _tiles) (`/Game/BP_Grid.CountBombsAndTiles` GameGrid))
  (`TextBlock.SetText` (`/Game/GameUI.MinesCount` _gameuiwidget) (`KismetTextLibrary.Conv_IntToText` _bombsremaining))
  (`TextBlock.SetText` (`/Game/GameUI.TilesCount` _gameuiwidget) (`KismetTextLibrary.Conv_IntToText` _tiles)))

(event `GameOver`
  (params (BombTile :type "/Game/Tile/BP_Tile Object Reference"))
  (`GameplayStatics.PlayWorldCameraShake` "/Game/CS_ExplosionShake.CS_ExplosionShake_C" (`self.K2_GetActorLocation` BombTile) 0.0 1000.0 0.0 true))

(fn `UserConstructionScript`)