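; Player controller for a Minesweeper game that handles tile selection by click or touch, plus pausing.
; Pressing Select on the current tile restarts a hold timer, and releasing passes the key and held time to that tile's Clicked.
; For tiles in one particular state, a cursor-following widget shows hold progress toward the reveal threshold through a dynamic material parameter updated on Tick.
; The Pause input calls PauseGame on the game mode.
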(event `self.ReceiveBeginPlay`
  ;[1 1 1] Create TimeHeld Widget and set up Material
  (bind _returnvalue (`|CreateWidget` "/Game/HoldTimer.HoldTimer_C"))
  (bind _output_get (set `self.HoldTimerWidget` _returnvalue))
  (`Widget.SetVisibility` _output_get "Collapsed")
  (`UserWidget.AddToViewport` _output_get 0)
  (bind _returnvalue_2 (`KismetMaterialLibrary.CreateDynamicMaterialInstance` "/Game/M_HoldTimer.M_HoldTimer"))
  (bind _output_get_2 (set `self.HoldTimerMaterial` _returnvalue_2))
  (`Image.SetBrushFromMaterial` (`/Game/HoldTimer.Image_0` (`self.HoldTimerWidget`)) _output_get_2))

(event `self.ReceiveTick`
  (params (DeltaSeconds :type "Float (single-precision)"))
  (bind (_locationx _locationy) (`self.GetMousePosition`))
  (bind _holdtimerwidget (`self.HoldTimerWidget`))
  ;[1 1 1] Track Touched Time
  (set `self.HoldTime` (+ (`self.HoldTime`) DeltaSeconds))
  ;[1 1 1] Have HoldTimeCircle follow mouse cursor
  (`UserWidget.SetPositionInViewport` _holdtimerwidget (- (`KismetMathLibrary.MakeVector2D` _locationx _locationy) (`Widget.GetDesiredSize` (`/Game/HoldTimer.Image_0` _holdtimerwidget))) true)
  (`MaterialInstanceDynamic.SetScalarParameterValue` (`self.HoldTimerMaterial`) "CompletionAmount" (`KismetMathLibrary.FClamp` (/ (`self.HoldTime`) (`self.TimeHeldForReveal`)))))

(event `InputAction|Select`
  (params (Key :type "Key Structure"))
  (bind _currenttile (`self.CurrentTile`))
  (bind _holdtimerwidget (`self.HoldTimerWidget`))
  (bind _currenttile_2 (`self.CurrentTile`))
  ;[1 1 1] Send Click/Touch Event with Held Time
  (:`Pressed`
    (if (`KismetSystemLibrary.IsValid` _currenttile_2)
      (set `self.HoldTime` 0.0)
      (set `self.Pressed` true)
      (if (`|EnumEquality` (`/Game/Tile/BP_Tile.TileState` _currenttile_2) "NewEnumerator0")
        (`Widget.SetVisibility` _holdtimerwidget "HitTestInvisible"))))
  (:`Released`
    (`Widget.SetVisibility` _holdtimerwidget "Collapsed")
    (`/Engine/EditorBlueprintResources/StandardMacros.IsValid` (`self.CurrentTile`)
      (:`Is Valid`
        (`/Game/Tile/BP_Tile.Clicked` _currenttile _currenttile Key (`self.HoldTime`))
        (set `self.Pressed` false)))))

(event `InputAction|Pause`
  (params (Key :type "Key Structure"))
  (:`Pressed`
    (if (not (`GameplayStatics.IsGamePaused`))
      (bind _asgm_minesweeper_2 (cast `/Game/GM_Minesweeper2` (`GameplayStatics.GetGameMode`)))
      (`/Game/GM_Minesweeper2.PauseGame` _asgm_minesweeper_2))))

(fn `UserConstructionScript`)