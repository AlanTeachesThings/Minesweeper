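; Minesweeper game mode that builds a match and resolves winning or losing.
; On BeginPlay it spawns BP_Grid from the size and bomb count in GI_Minesweeper, makes it the view target, enables mouse clicking and creates the GameUI.
; UpdateScores refreshes the mine and tile counters and declares a win when both reach zero.
; GameOver disables tiles, plays an explosion camera shake at the bomb and shows the loss widget.
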(event `self.ReceiveBeginPlay`
  (bind _returnvalue (`GameplayStatics.GetPlayerController` 0))
  (`WidgetBlueprintLibrary.SetInputMode_GameAndUIEx` (`GameplayStatics.GetPlayerController` 0) null)
  (bind _asgi_minesweeper (cast `/Game/GI_Minesweeper` (`GameplayStatics.GetGameInstance`)))
  ;[1 1 1] Spawn Grid
  (bind _returnvalue_2 (`|SpawnActorFromClass` "/Game/BP_Grid.BP_Grid_C" (`KismetMathLibrary.MakeTransform` (0.0 0.0 0.0)) "Undefined" "OverrideRootScale" null (`/Game/GI_Minesweeper.NewGridSize` _asgi_minesweeper) (100.0 100.0) (`/Game/GI_Minesweeper.NewGridBombCount` _asgi_minesweeper) null))
  ;[1 1 1] Set Up Camera
  (`PlayerController.SetViewTargetWithBlend` _returnvalue _returnvalue_2 0.0 "VTBlend_Linear" 0.0 false)
  ;[1 1 1] Set Up Mouse Input
  (set `PlayerController.bEnableMouseOverEvents` true _returnvalue)
  (set `PlayerController.bEnableClickEvents` true _returnvalue)
  (set `PlayerController.bShowMouseCursor` true _returnvalue)
  ;[1 1 1] Set up Game UI
  (bind _returnvalue_3 (`|CreateWidget` "/Game/UI/GameUI.GameUI_C"))
  (bind _output_get (set `self.GameUIWidget` _returnvalue_3))
  (`UserWidget.AddToViewport` _output_get 0)
  (bind _outactors (`GameplayStatics.GetAllActorsOfClass` "/Game/BP_Grid.BP_Grid_C"))
  (for _array_element _outactors
    (`self.UpdateScores` _array_element)))

(event `UpdateScores`
  (params (GameGrid :type "/Game/BP_Grid Object Reference"))
  (bind _gameuiwidget (`self.GameUIWidget`))
  ;[1 1 1] Update Scores
  (bind (_bombsremaining _tiles) (`/Game/BP_Grid.CountBombsAndTiles` GameGrid))
  (`TextBlock.SetText` (`/Game/UI/GameUI.MinesCount` _gameuiwidget) (`KismetTextLibrary.Conv_IntToText` _bombsremaining))
  (`TextBlock.SetText` (`/Game/UI/GameUI.TilesCount` _gameuiwidget) (`KismetTextLibrary.Conv_IntToText` _tiles))
  ;[1 1 1] Check for Win
  (if (and (== _bombsremaining 0) (== _tiles 0))
    (bind _outactors (`GameplayStatics.GetAllActorsOfClass` "/Game/BP_Grid.BP_Grid_C"))
    (for _array_element _outactors
      (`/Game/BP_Grid.DisableTiles` _array_element))
    (`self.GameWin`)))

(event `GameOver`
  (params (BombTile :type "/Game/Tile/BP_Tile Object Reference"))
  ;[1 1 1] Game Over
  (bind _outactors (`GameplayStatics.GetAllActorsOfClass` "/Game/BP_Grid.BP_Grid_C"))
  (for _array_element _outactors
    (`/Game/BP_Grid.DisableTiles` _array_element))
  (`GameplayStatics.PlayWorldCameraShake` "/Game/CS_ExplosionShake.CS_ExplosionShake_C" (`self.K2_GetActorLocation` BombTile) 0.0 1000.0 0.0 true)
  (bind _returnvalue (`|CreateWidget` "/Game/UI/GameOver.GameOver_C"))
  (`UserWidget.AddToViewport` _returnvalue 0))

(event `GameWin`
  ;[1 1 1] Game Win
  (bind _returnvalue (`|CreateWidget` "/Game/UI/GameWin.GameWin_C"))
  (`UserWidget.AddToViewport` _returnvalue 0))

(fn `UserConstructionScript`)