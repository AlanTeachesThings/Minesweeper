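; BP_Tile is one Minesweeper grid tile that tracks hidden, flagged or revealed state and whether it is a bomb.
; Short presses toggle a BP_Flag and long presses reveal; revealed tiles clear neighbours when flags match the bomb count, otherwise they pulse.
; Reveals explode bombs or flood-fill zeros through SpawningGrid, notifying the game mode.
; Timelines drive dynamic materials for hover highlight, number text and a segmented flag-progress indicator.
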(event `self.ReceiveBeginPlay`
  (bind _highlight (`self.Highlight`))
  ;[1 1 1] Master Clicked Functuion
  (`|ExecutionSequence`
    (:`then_0`
      ;[1 1 1] Set up HighlightMaterial
      (bind _returnvalue (`KismetMaterialLibrary.CreateDynamicMaterialInstance` "/Game/Tile/M_TileHighlight.M_TileHighlight"))
      (bind _output_get (set `self.HighlightMaterial` _returnvalue))
      (`PrimitiveComponent.SetMaterial` _highlight 0 _output_get)
      (`MeshComponent.SetScalarParameterValueOnMaterials` _highlight "Opacity" 0.0))
    (:`then_1`
      ;[1 1 1] Set up Text Material
      (bind _returnvalue_2 (`KismetMaterialLibrary.CreateDynamicMaterialInstance` "/Game/Tile/M_TileTextMaterial.M_TileTextMaterial"))
      (bind _output_get_2 (set `self.TextMaterial` _returnvalue_2))
      (`TextRenderComponent.SetTextMaterial` (`self.BombCountRender`) _output_get_2)
      (`MaterialInstanceDynamic.SetScalarParameterValue` _output_get_2 "Opacity" 0.0)
      (`MaterialInstanceDynamic.SetVectorParameterValue` _output_get_2 "Colour" (struct :`R` 1.0 :`G` 1.0 :`B` 1.0 :`A` 1.0)))
    (:`then_2`
      ;[1 1 1] Set up MarkCount Material
      (bind _returnvalue_3 (`KismetMaterialLibrary.CreateDynamicMaterialInstance` "/Game/Tile/M_TileMarkCount.M_TileMarkCount"))
      (bind _output_get_3 (set `self.MarkCountMaterial` _returnvalue_3))
      (`PrimitiveComponent.SetMaterial` (`self.MarkCountIndicator`) 0 _output_get_3)
      (`MaterialInstanceDynamic.SetScalarParameterValue` _output_get_3 "Opacity" 0.0)
      (`MaterialInstanceDynamic.SetScalarParameterValue` _output_get_3 "CompletionAmount" 0.0)
      (`MaterialInstanceDynamic.SetScalarParameterValue` _output_get_3 "Glow" 0.0))
    (:`then_3`
      ;[1 1 1] Bind Events
      (add `self.OnBeginCursorOver` (delegate `CursorOver`))
      (add `self.OnEndCursorOver` (delegate `CursorOut`)))))

(event `Clicked`
  (params (TouchedActor :type "Actor Object Reference") (ButtonPressed :type "Key Structure" :default "None") (PressedTime :type "Float (double-precision)"))
  (bind _tilestate (`self.TileState`))
  ;[1 1 1] Master Clicked Functuion
  (if (< PressedTime (`/Game/PC_MinesweeperController.TimeHeldForReveal` (cast `/Game/PC_MinesweeperController` (`GameplayStatics.GetPlayerController` 0) :!pure true)))
    ;;[1 1 1] Short Press
    (switch `/Game/Enum_TileState` _tilestate
      (:`NewEnumerator0`
        (`self.Mark`))
      (:`NewEnumerator1`
        (if (== (`self.BombsNearby`) (`self.MarksNearby`)) :!label _label
          (`/Game/BP_Grid.RevealSurroundingTiles` (`self.SpawningGrid`) (`self.GridPosition`))
          (else
            (bind (_direction _glow) (`Timeline|PulseMarkCount` :!via `PlayFromStart`)
              (:`Update`
                (`MaterialInstanceDynamic.SetScalarParameterValue` (`self.MarkCountMaterial`) "Glow" _glow))))))
      (:`NewEnumerator2`
        (`self.UnMark`)))
    (else
      ;;[1 1 1] Long Press
      (switch `/Game/Enum_TileState` _tilestate
        (:`NewEnumerator0`
          (`self.Reveal` 0.0))
        (:`NewEnumerator1`
          (goto _label))))))

(event `CursorOver` :!signature `self.OnBeginCursorOver`
  (params (TouchedActor :type "Actor Object Reference"))
  (bind _highlightmaterial (`self.HighlightMaterial`))
  ;[1 1 1] Cursor Over and Out
  (set `/Game/PC_MinesweeperController.CurrentTile` self (cast `/Game/PC_MinesweeperController` (`GameplayStatics.GetPlayerController` 0) :!pure true))
  (bind (_direction _opacity _glow) (`Timeline|RevealHighlight` :!label _label_2)
    (:`Update`
      (`MaterialInstanceDynamic.SetScalarParameterValue` _highlightmaterial "Opacity" _opacity)
      (`MaterialInstanceDynamic.SetScalarParameterValue` _highlightmaterial "Glow" _glow))))

(event `CursorOut` :!signature `self.OnEndCursorOver`
  (params (TouchedActor :type "Actor Object Reference"))
  ;[1 1 1] Cursor Over and Out
  (set `/Game/PC_MinesweeperController.CurrentTile` null (cast `/Game/PC_MinesweeperController` (`GameplayStatics.GetPlayerController` 0) :!pure true))
  (goto _label_2 :!via `Reverse`))

(event `MakeBomb`
  ;[1 1 1] Assign this tile as a bomb
  (set `self.isBomb` true)
  (`ActorComponent.K2_DestroyComponent` (`self.BombCountRender`))
  (`ActorComponent.K2_DestroyComponent` (`self.MarkCountIndicator`)))

(event `Mark`
  (bind _spawninggrid (`self.SpawningGrid`))
  ;[1 1 1] Mark With Flag
  (bind _returnvalue (`|SpawnActorFromClass` "/Game/Flag/BP_Flag.BP_Flag_C" (`KismetMathLibrary.MakeTransform` (`self.K2_GetActorLocation`)) "Undefined" "OverrideRootScale" null null))
  (bind _output_get (set `self.Flag` _returnvalue))
  (`/Game/Flag/BP_Flag.Enter` _output_get self)
  (set `self.TileState` "NewEnumerator2")
  (`/Game/BP_Grid.UpdateFlagCounts` _spawninggrid)
  (`/Game/GM_Minesweeper2.UpdateScores` (cast `/Game/GM_Minesweeper2` (`GameplayStatics.GetGameMode`) :!pure true) _spawninggrid))

(event `UnMark`
  (bind _spawninggrid (`self.SpawningGrid`))
  ;[1 1 1] Remove Flag
  (`/Game/Flag/BP_Flag.Leave` (`self.Flag`) self)
  (set `self.TileState` "NewEnumerator0")
  (`/Game/BP_Grid.UpdateFlagCounts` _spawninggrid)
  (`/Game/GM_Minesweeper2.UpdateScores` (cast `/Game/GM_Minesweeper2` (`GameplayStatics.GetGameMode`) :!pure true) _spawninggrid))

(event `Reveal`
  (params (Delay :type "Float (double-precision)"))
  (bind _grassparticles (`self.GrassParticles`))
  (bind _markcountmaterial (`self.MarkCountMaterial`))
  (bind _textmaterial (`self.TextMaterial`))
  ;[1 1 1] Reveal
  (if (`self.isBomb`)
    ;;[1 1 1] IS A BOMB
    (`ActorComponent.K2_DestroyComponent` (`self.GrassParticles`))
    (`PrimitiveComponent.SetMaterial` (`self.Plane`) 0 "/Game/Tile/M_DirtCrater.M_DirtCrater")
    (`ActorComponent.Activate` (`self.Explosion`) true)
    (`/Game/GM_Minesweeper2.GameOver` (cast `/Game/GM_Minesweeper2` (`GameplayStatics.GetGameMode`) :!pure true) self)
    (else
      (`KismetSystemLibrary.Delay` Delay)
      (if (`|EnumEquality` (`self.TileState`) "NewEnumerator0")
        (set `self.TileState` "NewEnumerator1")
        (`ActorComponent.Deactivate` _grassparticles)
        (`SceneComponent.SetVisibility` _grassparticles false false)
        (`ActorComponent.Activate` (`self.GrassBurst`) false)
        (`|ExecutionSequence`
          (:`then_0`
            (bind (_direction _opacity _glow) (`Timeline|RevealEffects` :!via `PlayFromStart`)
              (:`Update`
                (`|ExecutionSequence`
                  (:`then_0`
                    (`MaterialInstanceDynamic.SetScalarParameterValue` _textmaterial "Opacity" _opacity)
                    (`MaterialInstanceDynamic.SetScalarParameterValue` _textmaterial "Glow" _glow))
                  (:`then_1`
                    (`MaterialInstanceDynamic.SetScalarParameterValue` _markcountmaterial "Opacity" _opacity)
                    (`MaterialInstanceDynamic.SetScalarParameterValue` _markcountmaterial "Glow" _glow))))))
          (:`then_1`
            (`/Game/GM_Minesweeper2.UpdateScores` (cast `/Game/GM_Minesweeper2` (`GameplayStatics.GetGameMode`) :!pure true) (`self.SpawningGrid`))
            (if (== (`self.BombsNearby`) 0)
              (`/Game/BP_Grid.RevealSurroundingTiles` (`self.SpawningGrid`) (`self.GridPosition`)))))))))

(event `UpdateNumbers`
  (params (NumberOfNearbyBombs :type Integer))
  (bind _bombcountrender (`self.BombCountRender`))
  ;[1 1 1] Set everything related to the BombCount
  (bind _output_get (set `self.BombsNearby` NumberOfNearbyBombs))
  (if (> _output_get 0)
    (`/Engine/EditorBlueprintResources/StandardMacros.IsValid` _bombcountrender
      (:`Is Valid`
        (`TextRenderComponent.K2_SetText` _bombcountrender (`KismetTextLibrary.Conv_IntToText` NumberOfNearbyBombs))
        (`MaterialInstanceDynamic.SetScalarParameterValue` (`self.MarkCountMaterial`) "Segments" (`KismetMathLibrary.Conv_IntToDouble` NumberOfNearbyBombs))))
    (else
      (`ActorComponent.K2_DestroyComponent` _bombcountrender)
      (`ActorComponent.K2_DestroyComponent` (`self.MarkCountIndicator`)))))

(event `UpdateFlagCount`
  (params (FlagsFound :type Integer))
  ;[1 1 1] Update everything related to the number of nearby flags
  (bind _output_get (set `self.MarksNearby` FlagsFound))
  (`MaterialInstanceDynamic.SetScalarParameterValue` (`self.MarkCountMaterial`) "CompletionAmount" (/ (`KismetMathLibrary.Conv_IntToDouble` _output_get) (`KismetMathLibrary.Conv_IntToDouble` (`self.BombsNearby`)))))

(fn `UserConstructionScript`)